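; Cannon actor that fires a projectile at the player's head each time its ActivateEvent is triggered.
; The shot plays a Niagara effect and sound, then gets the player pawn's head location through the I_ProyectileObjective interface.
; A high-arc suggested velocity launches BP_Proyectil from the effect's location.
; A timeline, slowed on BeginPlay, then animates the Pivot's roll to move the cannon head.
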(event EventBeginPlay
  (Components|Timeline|SetPlayRate (Variables|Default|GetTL_AnimateHead) 0.5))

(event EventActivateEvent
  (bind _niagara (Variables|Default|GetNiagara))
  (bind _niagara_2 (Variables|Default|GetNiagara))
  (bind _returnvalue (Transformation|GetWorldLocation _niagara_2))
  (Components|Activation|Activate _niagara false)
  (Audio|PlaySoundatLocation "/Game/Sonido/SFX/Cannon/CannonShotCue.CannonShotCue" (Transformation|GetWorldLocation _niagara) "0, 0, 0" 1.0 1.0 0.0 0 0 0 0)
  (bind _asi_proyectile_objective (Utilities|Casting|CastToI_ProyectileObjective (Game|Player|GetPlayerPawn 0)))
  (bind _location (Default|GetHeadLocation _asi_proyectile_objective))
  (bind _outlaunchvelocity (Game|SuggestProjectileVelocityCustomArc _returnvalue _location 0.0 0.95))
  (Game|SpawnActorfromClass "/Game/VRTemplate/Blueprints/Proyectiles_/BP_Proyectil.BP_Proyectil_C" (Math|Transform|MakeTransform _returnvalue "0, 0, 0" "1.000000,1.000000,1.000000") "Undefined" "MultiplyWithRoot" 0 _outlaunchvelocity 0)
  (bind _alpha (Timeline|TL_AnimateHead PlayFromStart)
    (:Update
      (Transformation|SetRelativeRotation (Variables|Default|GetPivot) (Math|Rotator|MakeRotator (Math|Float|Lerp -2e+01 -65.0 _alpha) 0.0 0.0) false false))))

(fn ConstructionScript)